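; BP_Dodge is a pickup rune item whose side effect temporarily raises attack power after the owner dodges.
; While the effect is added, it listens to the owning CAttachment's state changes for Roll or BackStep.
; Each dodge releases any active boost before reapplying it on a five-second timer, so it refreshes without stacking.
; Destruction releases any pending boost, and LookAt supplies the pickup prompt from the item ID.
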(event Custom|SideEffect
  (params (InPrevType :type EStateType%20Enum :default "Idle") (InNewType :type EStateType%20Enum :default "Idle"))
  (if (or (Utilities|Enum|Equal(Enum) InNewType "Roll") (Utilities|Enum|Equal(Enum) InNewType "BackStep"))
    (if (Utilities|Time|IsValidTimerHandle (Variables|Default|GetHandle))
      (CallFunction|ReleaseSIdeEffect))
    (Class|CAttachmentStatusComponent|IncreasePower (Variables|Default|GetAttachmentStatus) 0.3)
    (bind _returnvalue (Utilities|Time|SetTimerbyEvent (delegate Custom|ReleaseSIdeEffect) 5.0))
    (Variables|Default|SetHandle _returnvalue)
    (Development|PrintString "회피 시 공격력증가 적용" true false)))

(event Custom|ReleaseSIdeEffect
  (Class|CAttachmentStatusComponent|DecreasePower (Variables|Default|GetAttachmentStatus) 0.3)
  (Utilities|Time|ClearandInvalidateTimerbyHandle (Variables|Default|GetHandle))
  (Variables|Default|SetHandle "")
  (Development|PrintString "회피 시 공격력증가 해제" true false))

(event EventAddSideEffect
  (bind _ascattachment (Utilities|Casting|CastToCAttachment (Components|GetOwner)))
  (bind _output_get (Variables|Default|SetOwnerAttachmentState (Variables|/Script/Game.CAttachment|GetState _ascattachment)))
  (EventDispatchers|BindEventtoOnStateTypeChanged _output_get (delegate Custom|SideEffect)))

(event EventRemoveSideEffect
  (EventDispatchers|UnbindEventfromOnStateTypeChanged (Variables|Default|GetOwnerAttachmentState) (delegate Custom|SideEffect)))

(event EventDestroyed
  (if (Utilities|Time|IsValidTimerHandle (Variables|Default|GetHandle))
    (CallFunction|ReleaseSIdeEffect)))

(fn ConstructionScript
  (Physics|SetSimulatePhysics (Variables|Default|GetItemMesh) false))

(fn Lookat
  (params (InActor :type Actor%20Object%20Reference))
  (return (Utilities|Text|FormatText "줍기 : {ItemID}" (.rowname (Variables|/Script/Game.CItemDataComponent|GetItemID (Variables|Default|GetCItemData))))))