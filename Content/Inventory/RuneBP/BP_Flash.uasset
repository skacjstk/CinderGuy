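; BP_Flash is an inventory rune item that shows a "줍기" (pick up) prompt with its item ID when looked at.
; Its construction script turns off physics on the item mesh.
; The add and remove side-effect events are empty.
; Disconnected graph logic would cache the owning CAttachment's state and raise or lower attack speed, but it never runs.
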(event EventAddSideEffect)

(event EventRemoveSideEffect)

(fn ConstructionScript
  (Physics|SetSimulatePhysics (Variables|Default|GetItemMesh) false))

(fn Lookat
  (params (InActor :type Actor%20Object%20Reference))
  (return (Utilities|Text|FormatText "줍기 : {ItemID}" (.rowname (Variables|/Script/Game.CItemDataComponent|GetItemID (Variables|Default|GetCItemData))))))