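; BP_CPlayer is a player Blueprint that adds keyboard test hotkeys for saving and restoring the character's position.
; NumPad 3 creates a BP_SaveGame object, stores the actor's current location in it and saves it asynchronously to the CPlayer slot.
; NumPad 1 loads that slot, casts it to BP_SaveGame and moves the actor to the stored location.
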(event EventBeginPlay)

(event Collision|EventActorBeginOverlap
  (params (OtherActor :type Actor%20Object%20Reference)))

(event Input|KeyboardEvents|NumPadOne
  (params (Key :type Key%20Structure :default "None"))
  (:Pressed
    (bind _returnvalue (SaveGame|LoadGamefromSlot "CPlayer"))
    (bind _asbp_save_game (Utilities|Casting|CastToBP_SaveGame _returnvalue))
    (Transformation|SetActorLocation (Variables|/Game/Objects/BP_SaveGame.BP_SaveGame_C|GetCharacterLastLocation _asbp_save_game) false false)))

(event Input|KeyboardEvents|NumPadThree
  (params (Key :type Key%20Structure :default "None"))
  (:Pressed
    (Development|PrintString "세이브 게임 호출")
    (bind _returnvalue (SaveGame|CreateSaveGameObject "/Game/Objects/BP_SaveGame.BP_SaveGame_C"))
    (bind _output_get (Variables|Default|SetSaveGameTest _returnvalue))
    (Variables|/Game/Objects/BP_SaveGame.BP_SaveGame_C|SetCharacterLastLocation _output_get (Transformation|GetActorLocation))
    (|AsyncSaveGametoSlot _output_get "CPlayer")))

(fn ConstructionScript)