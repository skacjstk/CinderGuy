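; Game mode that saves and restores the player's inventory and actions as the match state changes.
; On Leaving Map it creates a fresh BP_SaveGame, records the current level name plus the player's Action and Inventory components, and writes it to a fixed slot.
; On In Progress it loads that slot and passes the inventory and action data to BP_CPlayer, leaving the saved level unused.
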(event Custom|Save%20Game
  (bind _returnvalue (SaveGame|CreateSaveGameObject "/Game/Objects/BP_SaveGame.BP_SaveGame_C"))
  (|GameSaveNode _returnvalue)
  (SaveGame|SaveGametoSlot (Variables|Default|GetSaveGameObject) "CPlayer"))

(event Custom|Load%20Game
  (bind _returnvalue (SaveGame|LoadGamefromSlot "CPlayer"))
  (bind _asbp_save_game (Utilities|Casting|CastToBP_SaveGame _returnvalue))
  (bind (_playerinventorycontent _saveactionarray) (Default|LoadPlayerData _asbp_save_game))
  (bind _asbp_cplayer (Utilities|Casting|CastToBP_CPlayer (Game|GetPlayerCharacter 0)))
  (Default|LoadGamefromGameMode _asbp_cplayer _playerinventorycontent _saveactionarray))

(event EventOnSetMatchState
  (params (NewState :type Name :default "None"))
  (switch name NewState
    (:LeavingMap
      (CallFunction|SaveGame))
    (:InProgress
      (CallFunction|LoadGame))))

(fn ConstructionScript)