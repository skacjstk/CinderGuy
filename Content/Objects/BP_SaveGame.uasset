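; BP_SaveGame is a save-game object that stores and returns the player's last level, inventory and per-action attachment items.
; SavePlayerData walks every action type, appending non-empty attachment inventories to SaveAction, then copies the player inventory if it has items.
; SaveAction and the Test item-ID list are never cleared here, and placeholder test values are also written.
; LoadPlayerData returns the stored data with a zero player location, omitting the saved level.
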(fn SavePlayerData
  (params (LastLevel :type String) (ActionComponent :type C%20Action%20Component%20Object%20Reference) (Inventory :type C%20Inventory%20Component%20Object%20Reference))
  (bind _content (Variables|/Script/Game.CInventoryComponent|GetContent Inventory))
  (Variables|Default|SetPlayerLastLevel LastLevel)
  (Utilities|FlowControl|Sequence
    (:then_0
      (bind _enumvalue (|ForEachEActionType)
        (:LoopBody
          (Utilities|IsValid (Class|CActionComponent|GetDataObject ActionComponent (Math|Conversions|ToInteger(Byte) _enumvalue))
            (:Is%20Valid
              ;[1 1 1] 1개 이상 있을 때만 저장
              (Utilities|IsValid (Class|CActionObjectContainer|GetAttachment (Class|CActionComponent|GetDataObject ActionComponent (Math|Conversions|ToInteger(Byte) _enumvalue)))
                (:Is%20Valid
                  (if (Utilities|Array|IsValidIndex (Variables|/Script/Game.CInventoryComponent|GetContent (Class|CAttachment|GetAttachmentInventoryComponent (Class|CActionObjectContainer|GetAttachment (Class|CActionComponent|GetDataObject ActionComponent (Math|Conversions|ToInteger(Byte) _enumvalue))))))
                    (Utilities|Array|Add (Variables|Default|GetSaveAction) (Utilities|Struct|MakeSaveActionData _enumvalue (Variables|/Script/Game.CInventoryComponent|GetContent (Class|CAttachment|GetAttachmentInventoryComponent (Class|CActionObjectContainer|GetAttachment (Class|CActionComponent|GetDataObject ActionComponent (Math|Conversions|ToInteger(Byte) _enumvalue)))))))))))))))
    (:then_1
      (if (Utilities|Array|IsValidIndex _content)
        (bind _output_get (Variables|Default|SetSaveInventory _content))
        (for _array_element _output_get
          (Utilities|Array|Add (Variables|Default|GetTest) (.ItemID (Utilities|Struct|BreakSlot _array_element))))
        (Variables|Default|SetTestName "TestPlayer")
        (Variables|Default|SetTestInt 12)))))

(fn LoadPlayerData
  (return (Variables|Default|GetSaveInventory) (Variables|Default|GetSaveAction) (Variables|Default|GetTest) (Variables|Default|GetTestInt) (Variables|Default|GetTestName) ""))