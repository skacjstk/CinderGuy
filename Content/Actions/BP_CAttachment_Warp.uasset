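; BP_CAttachment_Warp is the attachment Blueprint for the Warp action, providing its visual components.
; Its Decal, SkeletalMesh and StaticMesh start hidden on BeginPlay, become visible on equip and hide again on unequip.
; Visibility changes apply to these three components without propagating to their children, and the Blueprint contains no warp logic itself.
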(event EventBeginPlay
  (Rendering|SetVisibility (Variables|Default|GetDecal) false false))

(event EventOnEquip
  (Rendering|SetVisibility (Variables|Default|GetDecal) true false))

(event EventOnUnequip
  (Rendering|SetVisibility (Variables|Default|GetDecal) false false))

(fn ConstructionScript)